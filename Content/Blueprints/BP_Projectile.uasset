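; BP_Projectile is a projectile with a sprite that plays a flipbook hit effect when it explodes.
; Its OnExplode override hides the sprite, zeroes Speed and plays the ProjectileHit flipbook once on HitEffect.
; When the flipbook finishes, it clears the effect and calls the parent OnExplode, deferring the inherited explosion handling until the animation ends.
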(event Custom|ExplodeFinished
  (Sprite|SetFlipbook (Variables|Default|GetHitEffect))
  (|CallParentFunction))

(event EventBeginPlay)

(event Collision|EventActorBeginOverlap
  (params (OtherActor :type Actor%20Object%20Reference)))

(event EventTick
  (params (DeltaSeconds :type Float%20%28single-precision%29)))

(event EventOnExplode
  (bind _hiteffect (Variables|Default|GetHitEffect))
  (Rendering|SetVisibility (Variables|Default|GetProjectileSprite) false false)
  (Variables|Default|SetSpeed 0.0)
  (Sprite|SetFlipbook _hiteffect "/Game/ProjectileHit.ProjectileHit")
  (Audio|Components|Audio|Play _hiteffect)
  (Components|Timeline|SetLooping _hiteffect false)
  (EventDispatchers|BindEventtoOnFinishedPlaying _hiteffect (delegate Custom|ExplodeFinished)))

(fn ConstructionScript)